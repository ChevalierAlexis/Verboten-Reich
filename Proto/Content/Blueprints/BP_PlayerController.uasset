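; Player controller that relays movement, look, interaction, choice and rotate inputs through event dispatchers and manages the on-screen UI.
; BeginPlay creates the HUD and binds movement and look handlers, which drive the player pawn along control yaw or rotate the view.
; EnterDialog unbinds movement and interaction; Exit_Dialog rebinds movement and look and notifies the current interaction.
; ChangeUI swaps one active widget between HUD, dialogue, choice, examine, text and death screens.
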(event `InputAxis|MoveForward` :overrideparent false
  (params (AxisValue :type "Float (single-precision)"))
  (`self.OnMoveForward` AxisValue))

(event `OnMoveForwardEvent` :!signature `self.OnMoveForward`
  (params (AxisValue :type "Float (double-precision)"))
  (bind _returnvalue (`GameplayStatics.GetPlayerPawn` 0))
  (`/Engine/EditorBlueprintResources/StandardMacros.IsValid` _returnvalue
    (:`Is Valid`
      (`Pawn.AddMovementInput` _returnvalue (`KismetMathLibrary.GetForwardVector` (`KismetMathLibrary.MakeRotator` 0.0 0.0 (.yaw (`self.GetControlRotation`)))) AxisValue false))))

(event `InputAxis|MoveRight` :overrideparent false
  (params (AxisValue :type "Float (single-precision)"))
  (`self.OnMoveRight` AxisValue))

(event `MoveRightEvent` :!signature `self.OnMoveRight`
  (params (AxisValue :type "Float (double-precision)"))
  (bind _returnvalue (`GameplayStatics.GetPlayerPawn` 0))
  (`/Engine/EditorBlueprintResources/StandardMacros.IsValid` _returnvalue
    (:`Is Valid`
      (`Pawn.AddMovementInput` _returnvalue (`KismetMathLibrary.GetRightVector` (`KismetMathLibrary.MakeRotator` 0.0 0.0 (.yaw (`self.GetControlRotation`)))) AxisValue false))))

(event `self.ReceiveBeginPlay`
  (add `self.OnMoveRight` (`|CreateDelegate` :!event `MoveRightEvent`))
  (add `self.OnMoveForward` (`|CreateDelegate` :!event `OnMoveForwardEvent`))
  (add `self.OnExitDialogue` (`|CreateDelegate` :!event `Exit_Dialog`))
  (add `self.OnTurn` (`|CreateDelegate` :!event `TurnInput`))
  (add `self.OnPitch` (`|CreateDelegate` :!event `PitchEvent`))
  (add `self.GamepadOnPitch` (`|CreateDelegate` :!event `GamepadOnPitchEvent`))
  (add `self.GamepadOnTurn` (`|CreateDelegate` :!event `GamepaOnTurnEvent`))
  (bind _returnvalue (`|CreateWidget` "/Game/Blueprints/UI/W_HUD.W_HUD_C" (`GameplayStatics.GetPlayerController` 0)))
  (bind _output_get (set `self.Used_Interface` _returnvalue))
  (`UserWidget.AddToViewport` _output_get 0))

(event `Exit_Dialog`
  (set `self.Is_Dialog` false)
  (`self.ChangeUI` "NewEnumerator0")
  (add `self.OnMoveForward` (`|CreateDelegate` :!event `OnMoveForwardEvent`))
  (add `self.OnMoveRight` (`|CreateDelegate` :!event `MoveRightEvent`))
  (add `self.OnTurn` (`|CreateDelegate` :!event `TurnInput`))
  (add `self.OnPitch` (`|CreateDelegate` :!event `PitchEvent`))
  (add `self.GamepadOnPitch` (`|CreateDelegate` :!event `GamepadOnPitchEvent`))
  (add `self.GamepadOnTurn` (`|CreateDelegate` :!event `GamepaOnTurnEvent`))
  (if (not (== (`self.Current_Interaction`) null))
    (`/Game/Blueprints/BP_Interactions.Interaction_Exit_Dialogue` (`self.Current_Interaction`))))

(event `InputAction|Interact`
  (params (Key :type "Key Structure"))
  (:`Pressed`
    (`self.OnInteraction`)))

(event `InputAxis|LookUp` :overrideparent false
  (params (AxisValue :type "Float (single-precision)"))
  (`self.OnTurn`))

(event `TurnInput`
  (bind _returnvalue (`GameplayStatics.GetPlayerCharacter` 0))
  (`/Engine/EditorBlueprintResources/StandardMacros.IsValid` _returnvalue
    (:`Is Valid`
      (`Pawn.AddControllerPitchInput` _returnvalue (stale `InputAxis|LookUp` AxisValue)))))

(event `InputAction|FauxForward`
  (params (Key :type "Key Structure"))
  (:`Pressed`
    (`self.OnChoiceUp`)))

(event `InputAxis|Turn` :overrideparent false
  (params (AxisValue :type "Float (single-precision)"))
  (`self.OnPitch`))

(event `PitchEvent`
  (bind _returnvalue (`GameplayStatics.GetPlayerCharacter` 0))
  (`/Engine/EditorBlueprintResources/StandardMacros.IsValid` _returnvalue
    (:`Is Valid`
      (`Pawn.AddControllerYawInput` _returnvalue (stale `InputAxis|Turn` AxisValue)))))

(event `InputAction|FauxBackWard`
  (params (Key :type "Key Structure"))
  (:`Pressed`
    (`self.OnChoiceDown`)))

(event `InputAxis|LookUpRate`
  (params (AxisValue :type "Float (single-precision)"))
  (`self.GamepadOnPitch`))

(event `GamepadOnPitchEvent`
  (bind _returnvalue (`GameplayStatics.GetPlayerCharacter` 0))
  (`/Engine/EditorBlueprintResources/StandardMacros.IsValid` _returnvalue
    (:`Is Valid`
      (`Pawn.AddControllerPitchInput` _returnvalue (* (stale `InputAxis|LookUpRate` AxisValue) (`self.BaseLookUpRate`) (`GameplayStatics.GetWorldDeltaSeconds`))))))

(event `InputAction|FauxLeft`
  (params (Key :type "Key Structure"))
  (:`Pressed`
    (`self.Rotate` 0.0)))

(event `InputAxis|TurnRate`
  (params (AxisValue :type "Float (single-precision)"))
  (`self.GamepadOnTurn`))

(event `GamepaOnTurnEvent`
  (bind _returnvalue (`GameplayStatics.GetPlayerCharacter` 0))
  (`/Engine/EditorBlueprintResources/StandardMacros.IsValid` _returnvalue
    (:`Is Valid`
      (`Pawn.AddControllerYawInput` _returnvalue (* (stale `InputAxis|TurnRate` AxisValue) (`self.BaseTurnRate`) (`GameplayStatics.GetWorldDeltaSeconds`))))))

(event `InputAction|FauxRight`
  (params (Key :type "Key Structure"))
  (:`Pressed`
    (`self.Rotate` (stale `InputAxis|TurnRate` AxisValue))))

(fn `ChangeUI`
  (params (Selection :type "/Game/Data/E_UI Enum" :default "NewEnumerator0"))
  (switch `/Game/Data/E_UI` Selection
    (:`NewEnumerator0`
      (`Widget.RemoveFromParent` (`self.Used_Interface`))
      (set `self.Used_Interface` null)
      (bind _returnvalue (`|CreateWidget` "/Game/Blueprints/UI/W_HUD.W_HUD_C" (`GameplayStatics.GetPlayerController` 0)))
      (`UserWidget.AddToViewport` _returnvalue 0)
      (set `self.Used_Interface` _returnvalue))
    (:`NewEnumerator1`
      (`Widget.RemoveFromParent` (`self.Used_Interface`))
      (set `self.Used_Interface` null)
      (bind _returnvalue_2 (`|CreateWidget` "/Game/Blueprints/UI/W_Dialogue.W_Dialogue_C" (`GameplayStatics.GetPlayerController` 0)))
      (`UserWidget.AddToViewport` _returnvalue_2 0)
      (set `self.Used_Interface` _returnvalue_2))
    (:`NewEnumerator2`
      (`Widget.RemoveFromParent` (`self.Used_Interface`))
      (set `self.Used_Interface` null)
      (bind _returnvalue_3 (`|CreateWidget` "/Game/Blueprints/UI/W_Choix.W_Choix_C" (`GameplayStatics.GetPlayerController` 0)))
      (`UserWidget.AddToViewport` _returnvalue_3 0)
      (set `self.Used_Interface` _returnvalue_3))
    (:`NewEnumerator3`
      (`Widget.RemoveFromParent` (`self.Used_Interface`))
      (set `self.Used_Interface` null)
      (bind _returnvalue_4 (`|CreateWidget` "/Game/Blueprints/UI/W_Examine.W_Examine_C" (`GameplayStatics.GetPlayerController` 0)))
      (`UserWidget.AddToViewport` _returnvalue_4 0)
      (set `self.Used_Interface` _returnvalue_4))
    (:`NewEnumerator4`
      (`Widget.RemoveFromParent` (`self.Used_Interface`))
      (set `self.Used_Interface` null)
      (bind _returnvalue_5 (`|CreateWidget` "/Game/Blueprints/UI/W_Textes.W_Textes_C" (`GameplayStatics.GetPlayerController` 0)))
      (`UserWidget.AddToViewport` _returnvalue_5 0)
      (set `self.Used_Interface` _returnvalue_5))
    (:`NewEnumerator5`
      (`Widget.RemoveFromParent` (`self.Used_Interface`))
      (set `self.Used_Interface` null)
      (bind _returnvalue_6 (`|CreateWidget` "/Game/Blueprints/UI/W_Death.W_Death_C" (`GameplayStatics.GetPlayerController` 0)))
      (`UserWidget.AddToViewport` _returnvalue_6 0)
      (set `self.Used_Interface` _returnvalue_6))))

(fn `EnterDialog`
  (set `self.Is_Dialog` true)
  (`self.ChangeUI` "NewEnumerator1")
  (clear `self.OnMoveForward`)
  (clear `self.OnMoveRight`)
  (clear `self.OnInteraction`)
  (clear `self.OnMoveBackward`))

(fn `UserConstructionScript`)