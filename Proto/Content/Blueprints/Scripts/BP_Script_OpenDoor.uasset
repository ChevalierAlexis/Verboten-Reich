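; Interaction script for a hinged door that toggles open and closed, and can trigger a game over when opened.
; PlayScript flips the Open flag and plays or reverses a timeline that drives the Pivot's yaw.
; Opening with the player controller's Suspicion at threshold or above plays the LS_BulletDeath sequence and sets GameOver on the game instance.
; Tick polls that sequence player and loads the "Cellule" level once playback stops.
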(event `OnDoorOpen`
  (bind (_direction _newtrack_0) (`Timeline|Timeline_0` :!label _label)
    (:`Update`
      (`SceneComponent.K2_SetRelativeRotation` (`self.Pivot`) (`KismetMathLibrary.MakeRotator` 0.0 0.0 _newtrack_0) false false))))

(event `self.ReceiveActorBeginOverlap`
  (params (OtherActor :type "Actor Object Reference"))
  (`parent.ReceiveActorBeginOverlap` OtherActor))

(event `OnDoorClose`
  (goto _label :!via `Reverse`))

(event `self.ReceiveTick`
  (params (DeltaSeconds :type "Float (single-precision)"))
  (`parent.ReceiveTick` DeltaSeconds)
  (if (!= (`self.Is_Playing`) null)
    (if (not (`MovieSceneSequencePlayer.IsPlaying` (`self.Is_Playing`)))
      (`GameplayStatics.OpenLevel` "Cellule"))))

(fn `PlayScript`
  (`parent.PlayScript`)
  (if (`self.Open`)
    (`self.OnDoorClose`)
    (set `self.Open` false)
    (else
      (`self.OnDoorOpen`)
      (set `self.Open` true)
      (if (>= (`/Game/Blueprints/BP_PlayerController.Suspicion` (`/Game/Blueprints/BPFL_MainFunctionLibrary.CastToPlayerController`)) 10.0)
        (bind (_outactor _returnvalue) (`LevelSequencePlayer.CreateLevelSequencePlayer` "/Game/Animations/Level_Sequences/Scene1/LS_BulletDeath.LS_BulletDeath" (make `MovieSceneSequencePlaybackSettings` false (struct) 1.0 0.0 false false true true)))
        (`MovieSceneSequencePlayer.Play` _returnvalue)
        (set `self.Is_Playing` _returnvalue)
        (bind _asbp_game_instance (cast `/Game/Blueprints/BP_Game_Instance` (`GameplayStatics.GetGameInstance`)))
        (set `/Game/Blueprints/BP_Game_Instance.GameOver` true _asbp_game_instance)))))

(fn `UserConstructionScript`
  (`parent.UserConstructionScript`))