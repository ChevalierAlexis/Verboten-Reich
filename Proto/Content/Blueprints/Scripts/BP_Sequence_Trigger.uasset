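; BP_Sequence_Trigger is a box trigger that plays an assigned Level Sequence when the player enters it, sized by BoxTriggerSize in the construction script.
; On first overlap it sets DialogueDone, then requires BP_Player and BP_PlayerController casts before creating and playing the sequence player.
; Because the flag precedes the casts, any actor's overlap uses up the trigger; later overlaps only print a debug message.
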(event `self.ReceiveActorBeginOverlap`
  (params (OtherActor :type "Actor Object Reference"))
  (if (`self.DialogueDone`)
    (`KismetSystemLibrary.PrintString` "Can't change that now")
    (else
      (set `self.DialogueDone` true)
      (bind _asbp_player (cast `/Game/Blueprints/BP_Player` OtherActor))
      (cast `/Game/Blueprints/BP_PlayerController` (`self.GetInstigatorController` _asbp_player))
      (bind (_outactor _returnvalue) (`LevelSequencePlayer.CreateLevelSequencePlayer` (`self.Sequence_To_Play`)))
      (`MovieSceneSequencePlayer.Play` _returnvalue))))

(fn `UserConstructionScript`
  (`BoxComponent.SetBoxExtent` (`self.Box`) (`self.Box_Trigger_Size`) true))