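; Broken dialogue manager Blueprint that steps through DT_Dialogue rows by index, using row names cached on BeginPlay.
; PlayDialog puts the player controller into dialogue and binds its interaction event; two-option choices rebind input and jump to the chosen row.
; DialogLoop only checks for a single BP_Conditions actor.
; Its row lookup, text display, suspicion gain, choice trigger and exit logic are disconnected and never run.
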(event `self.ReceiveBeginPlay`
  (bind _outrownames (`DataTableFunctionLibrary.GetDataTableRowNames` "/Game/Data/DT_Dialogue.DT_Dialogue"))
  (for _array_element _outrownames
    (`KismetArrayLibrary.Array_AddUnique` (`self.Dialog_Array`) _array_element)))

(event `Continue_Dialogue`
  (set `self.Index_Dialog` (+ (`self.Index_Dialog`) 1))
  (`self.DialogLoop`))

(event `Choice_Up`
  (bind _asbp_player_controller (`self.CastToPlayerController`))
  (for (_array_element _array_index) (`self.Dialog_Array`)
    (if (== _array_element (`.RowName` (break `DataTableRowHandle` (`.Choix_1_2_0BAF7B8947E27EB294F2748403B22644` (break `/Game/Data/F_Choix` (`.Choix_59_F0A7C4244B9AADC7965648BFA82E1636` (break `` (struct))))))))
      (bind _output_get (set `self.Index_Dialog` _array_index))
      (`KismetSystemLibrary.PrintString` (`KismetStringLibrary.Conv_IntToString` _output_get))))
  (add `self.OnInteraction` _asbp_player_controller (delegate `Continue_Dialogue`))
  (clear `self.OnChoiceUp` _asbp_player_controller)
  (clear `self.OnChoiceDown` _asbp_player_controller)
  (`self.ChangeUI` _asbp_player_controller 0)
  (`self.DialogLoop`))

(event `Choice_Down`
  (bind _asbp_player_controller (`self.CastToPlayerController`))
  (for (_array_element _array_index) (`self.Dialog_Array`)
    (if (== _array_element (`.RowName` (break `DataTableRowHandle` (`.Choix_2_4_E9045C074A895E2B67DE87934F5B3924` (break `/Game/Data/F_Choix` (`.Choix_59_F0A7C4244B9AADC7965648BFA82E1636` (break `` (struct))))))))
      (set `self.Index_Dialog` _array_index)))
  (add `self.OnInteraction` _asbp_player_controller (delegate `Continue_Dialogue`))
  (clear `self.OnChoiceUp` _asbp_player_controller)
  (clear `self.OnChoiceDown` _asbp_player_controller)
  (`self.ChangeUI` _asbp_player_controller 0)
  (`self.DialogLoop`))

(fn `Choix`
  (bind (_texte_dialogue _interlocutor _choix) (break `` (struct)))
  (bind (_choix_1 _choix_2 _texte_1 _texte_2) (break `/Game/Data/F_Choix` _choix))
  (bind _asbp_player_controller (cast `` (`GameplayStatics.GetPlayerController` 0)))
  (clear `self.OnInteraction` _asbp_player_controller)
  (`self.ChangeUI` _asbp_player_controller 0)
  (bind _asw_choix (cast `` (`/Game/Blueprints/BP_Dialogue_Cassé.Used_Interface` _asbp_player_controller)))
  (`self.Set_Text_Choice_Up` _asw_choix _texte_1)
  (`self.Set_Text_Choice_Down` _asw_choix _texte_2)
  (`self.Set_Name_Text_Choice` _asw_choix _interlocutor)
  (`self.Set_Main_Text_Choice` _asw_choix _texte_dialogue)
  (add `self.OnChoiceUp` _asbp_player_controller (`|CreateDelegate` :!event `Choice_Up`))
  (add `self.OnChoiceDown` _asbp_player_controller (`|CreateDelegate` :!event `Choice_Down`)))

(fn `DialogLoop`
  (bind _asbp_game_instance (cast `/Game/FirstPersonBP/BP_Game_Instance` (`GameplayStatics.GetGameInstance`)))
  (bind _outactors (`GameplayStatics.GetAllActorsOfClass` "/Game/FirstPersonBP/BP_Conditions.BP_Conditions_C"))
  (if (`KismetArrayLibrary.Array_IsValidIndex` _outactors)
    (if (> (`KismetArrayLibrary.Array_Length` _outactors) 1)
      (`KismetSystemLibrary.PrintString` "Trop de BP Condition dans ce niveau !"))
    (else
      (`KismetSystemLibrary.PrintString` "Pas de BP Condition dans ce niveau"))))

(fn `PlayDialog`
  (params (DialogLine :type "DataTableRowHandle Structure"))
  (bind _asbp_player_controller (`self.CastToPlayerController`))
  (set `self.End` false)
  (`self.EnterDialog` _asbp_player_controller)
  (add `self.OnInteraction` _asbp_player_controller (`|CreateDelegate` :!event `Continue_Dialogue`))
  (for (_array_element _array_index) (`self.Dialog_Array`)
    (if (== _array_element (`.RowName` (break `DataTableRowHandle` DialogLine)))
      (set `self.Index_Dialog` _array_index)))
  (`self.DialogLoop`))

(fn `UserConstructionScript`)