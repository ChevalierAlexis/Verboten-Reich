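; Placeable interaction trigger, sized by BoxSize, that launches a dialogue, script, object examination or spy dialogue.
; While active, overlap binds Interact to the player controller's interaction event and, if input is needed, sets the HUD icon; otherwise dialogues and scripts play immediately.
; Dialogue and examination use the level's single BP_Dialogue or BP_Studio, printing French setup errors.
; Examining can flip a boolean condition in the game instance.
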(event `self.ReceiveBeginPlay`)

(event `Interact`
  (bind _condition (`self.Condition`))
  (if (`self.IsDialogue`)
    (`self.ScriptToLaunch`
      (:`then`
        (`KismetSystemLibrary.PrintString` "Tu ne peux pas mettre un dialogue et un script sur la même interaction !"))
      (:`else`
        (bind _outactors (`GameplayStatics.GetAllActorsOfClass` "/Game/Blueprints/BP_Dialogue.BP_Dialogue_C"))
        (if (`KismetArrayLibrary.Array_IsValidIndex` _outactors)
          (if (> (`KismetArrayLibrary.Array_Length` _outactors) 1)
            (`KismetSystemLibrary.PrintString` "Trop de BP Dialogue dans ce niveau !")
            (else
              (`/Game/Blueprints/BP_Dialogue.PlayDialog` (`|GetArrayItem` _outactors) (`self.DialogToLaunch`))))
          (else
            (`KismetSystemLibrary.PrintString` "Pas de BP Dialogue dans ce niveau")))))
    (else
      (bind _scripttolaunch (`self.ScriptToLaunch`)
        (:`then`
          (`/Game/Blueprints/Scripts/BP_Script.PlayScript` _scripttolaunch))
        (:`else`
          (`self.ObjectToExamine`
            (:`then`
              (bind _outactors_2 (`GameplayStatics.GetAllActorsOfClass` "/Game/Blueprints/BP_Studio.BP_Studio_C"))
              (if (`KismetArrayLibrary.Array_IsValidIndex` _outactors_2)
                (if (> (`KismetArrayLibrary.Array_Length` _outactors_2) 1)
                  (`KismetSystemLibrary.PrintString` "Trop de BP Studio dans ce niveau !")
                  (else
                    (bind _output (`|GetArrayItem` _outactors_2))
                    (`StaticMeshComponent.SetStaticMesh` (`/Game/Blueprints/BP_Studio.ItemToFocus` _output) (`self.ObjectToExamine`))
                    (`/Game/Blueprints/BP_Studio.Examine` _output)
                    (if (`self.IsCondition`)
                      (bind _asbp_game_instance (cast `/Game/Blueprints/BP_Game_Instance` (`GameplayStatics.GetGameInstance`)))
                      (set `self.Temp_Identifier` _condition)
                      (bind _dict_conditions (`/Game/Blueprints/BP_Game_Instance.Dict_Conditions` _asbp_game_instance))
                      (`BlueprintMapLibrary.Map_Remove` _dict_conditions _condition)
                      (bind (_condition_2 _boolean_value _numerical_value _if_false) (break `/Game/Data/F_Conditions` (`BlueprintMapLibrary.Map_Find` _dict_conditions _condition)))
                      (`BlueprintMapLibrary.Map_Add` _dict_conditions (`self.Temp_Identifier`) (make `/Game/Data/F_Conditions` _condition_2 (not _boolean_value) _numerical_value _if_false)))))
                (else
                  (`KismetSystemLibrary.PrintString` "Pas de BP Studio dans ce niveau"))))
            (:`else`
              (`KismetSystemLibrary.PrintString` "Pas de Script ou d'objet à examiner valide !"))))))))

(event `self.ReceiveActorBeginOverlap`
  (params (OtherActor :type "Actor Object Reference"))
  (if (`self.IsActive`)
    (bind _asbp_player_controller (cast `/Game/Blueprints/BP_PlayerController` (`self.GetInstigatorController` OtherActor)))
    (set `/Game/Blueprints/BP_PlayerController.Current_Interaction` self _asbp_player_controller)
    (add `/Game/Blueprints/BP_PlayerController.OnInteraction` _asbp_player_controller (delegate `Interact`))
    (switch `/Game/Data/E_Interactions` (`self.Selection`)
      (:`NewEnumerator0`
        (if (`self.NeedInteraction`)
          (set `self.IsDialogue` true)
          (bind _asw_hud (cast `/Game/Blueprints/UI/W_HUD` (`/Game/Blueprints/BP_PlayerController.Used_Interface` _asbp_player_controller)))
          (`/Game/Blueprints/UI/W_HUD.Set_Context_Image` _asw_hud "/Game/Textures/Textures/UI/talk.talk")
          (else
            (bind _outactors (`GameplayStatics.GetAllActorsOfClass` "/Game/Blueprints/BP_Dialogue.BP_Dialogue_C"))
            (if (`KismetArrayLibrary.Array_IsValidIndex` _outactors)
              (if (> (`KismetArrayLibrary.Array_Length` _outactors) 1)
                (`KismetSystemLibrary.PrintString` "Trop de BP Dialogue dans ce niveau !")
                (else
                  (`/Game/Blueprints/BP_Dialogue.PlayDialog` (`|GetArrayItem` _outactors) (`self.DialogToLaunch`))))))))
      (:`NewEnumerator2`
        (if (`self.NeedInteraction`)
          (bind _asw_hud_2 (cast `/Game/Blueprints/UI/W_HUD` (`/Game/Blueprints/BP_PlayerController.Used_Interface` _asbp_player_controller)))
          (`/Game/Blueprints/UI/W_HUD.Set_Context_Image` _asw_hud_2 "/Game/Textures/Textures/UI/Interact.Interact")
          (else
            (bind _scripttolaunch (`self.ScriptToLaunch`)
              (:`then`
                (`/Game/Blueprints/Scripts/BP_Script.PlayScript` _scripttolaunch))
              (:`else`
                (`KismetSystemLibrary.PrintString` "Il n'y a pas de script ou de dialogue lié à cette interaction !"))))))
      (:`NewEnumerator1`
        (if (`self.NeedInteraction`)
          (bind _asw_hud_3 (cast `/Game/Blueprints/UI/W_HUD` (`/Game/Blueprints/BP_PlayerController.Used_Interface` _asbp_player_controller)))
          (`/Game/Blueprints/UI/W_HUD.Set_Context_Image` _asw_hud_3 "/Game/Textures/Textures/UI/Interact.Interact")))
      (:`NewEnumerator3`
        (if (`self.NeedInteraction`)
          (set `self.IsDialogue` true)
          (bind _asw_hud_4 (cast `/Game/Blueprints/UI/W_HUD` (`/Game/Blueprints/BP_PlayerController.Used_Interface` _asbp_player_controller)))
          (`/Game/Blueprints/UI/W_HUD.Set_Context_Image` _asw_hud_4 "/Game/Textures/Textures/UI/human-earbckground-removebg-preview.human-earbckground-removebg-preview")
          (else
            (bind _outactors_2 (`GameplayStatics.GetAllActorsOfClass` "/Game/Blueprints/BP_Dialogue.BP_Dialogue_C"))
            (if (`KismetArrayLibrary.Array_IsValidIndex` _outactors_2)
              (if (> (`KismetArrayLibrary.Array_Length` _outactors_2) 1)
                (`KismetSystemLibrary.PrintString` "Trop de BP Dialogue dans ce niveau !")
                (else
                  (`/Game/Blueprints/BP_Dialogue.PlayDialog` (`|GetArrayItem` _outactors_2) (`self.DialogToLaunch`)))))))))))

(event `Interaction_Exit_Dialogue`
  (clear `/Game/Blueprints/BP_PlayerController.OnInteraction` (stale `self.ReceiveActorBeginOverlap` _asbp_player_controller))
  (add `/Game/Blueprints/BP_PlayerController.OnInteraction` (stale `self.ReceiveActorBeginOverlap` _asbp_player_controller) (delegate `Interact`)))

(event `self.ReceiveActorEndOverlap`
  (params (OtherActor :type "Actor Object Reference"))
  (set `self.IsDialogue` false)
  (bind _asbp_player_controller (cast `/Game/Blueprints/BP_PlayerController` (`GameplayStatics.GetPlayerController` 0)))
  (bind _asw_hud (cast `/Game/Blueprints/UI/W_HUD` (`/Game/Blueprints/BP_PlayerController.Used_Interface` _asbp_player_controller)))
  (`/Game/Blueprints/UI/W_HUD.Set_Context_Image` _asw_hud "/Game/Textures/Textures/UI/Target.Target")
  (clear `/Game/Blueprints/BP_PlayerController.OnInteraction` _asbp_player_controller))

(fn `UserConstructionScript`
  (`BoxComponent.SetBoxExtent` (`self.Box`) (`self.Box_Size`) true))