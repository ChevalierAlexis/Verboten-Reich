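; BP_PNJ is an NPC whose skeletal mesh and name come from a selected DT_Characters row at construction.
; Every Tick it line-traces forward from its capsule to detect the player.
; If the player it hits is using the Examine or Textes interface, or is in dialog during a Spy interaction, a delayed sequence exits the dialog and briefly shows a HUD text.
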(event `self.ReceiveTick`
  (params (DeltaSeconds :type "Float (single-precision)"))
  (bind _asbp_player_controller (`/Game/Blueprints/BPFL_MainFunctionLibrary.CastToPlayerController`))
  (bind _capsulecomponent (`self.CapsuleComponent`))
  (bind _returnvalue (`SceneComponent.K2_GetComponentLocation` _capsulecomponent))
  (bind _outhit (`KismetSystemLibrary.LineTraceSingle` _returnvalue (+ _returnvalue (* (`KismetMathLibrary.GetForwardVector` (`SceneComponent.K2_GetComponentRotation` _capsulecomponent)) 25000.0)) "TraceTypeQuery2"))
  (bind _asbp_player (cast `/Game/Blueprints/BP_Player` (`.HitActor` (`GameplayStatics.BreakHitResult` _outhit))))
  (bind _asbp_player_controller_2 (cast `/Game/Blueprints/BP_PlayerController` (`self.GetInstigatorController` _asbp_player)))
  (bind _used_interface (`/Game/Blueprints/BP_PlayerController.Used_Interface` _asbp_player_controller_2))
  (cast `/Game/Blueprints/UI/W_Examine` _used_interface
    (:`then`
      (`KismetSystemLibrary.Delay` 2.0 :!label _label)
      (`/Game/Blueprints/BP_PlayerController.Exit_Dialog` _asbp_player_controller)
      (bind _asw_hud (cast `/Game/Blueprints/UI/W_HUD` (`/Game/Blueprints/BP_PlayerController.Used_Interface` _asbp_player_controller)))
      (bind _textblock_0 (`/Game/Blueprints/UI/W_HUD.TextBlock_0` _asw_hud))
      (`TextBlock.SetOpacity` _textblock_0 1.0)
      (`KismetSystemLibrary.Delay` 3.0)
      (`TextBlock.SetOpacity` _textblock_0 0.0))
    (:`CastFailed`
      (cast `/Game/Blueprints/UI/W_Textes` _used_interface
        (:`then`
          (goto _label))
        (:`CastFailed`
          (bind _current_interaction (`/Game/Blueprints/BP_PlayerController.Current_Interaction` _asbp_player_controller_2))
          (if (!= _current_interaction null)
            (switch `/Game/Data/E_Interactions` (`/Game/Blueprints/BP_Interactions.Selection` _current_interaction)
              (:`NewEnumerator3`
                (if (`/Game/Blueprints/BP_PlayerController.Is_Dialog` _asbp_player_controller)
                  (goto _label))))))))))

(fn `UserConstructionScript`
  (bind (_datatable _rowname) (break `DataTableRowHandle` (`self.Character_Selected`)))
  (bind _returnvalue (`|GetDataTableRow` "/Game/Data/DT_Characters.DT_Characters" _rowname)
    (:`then`
      (`SkinnedMeshComponent.SetSkinnedAssetAndUpdate` (`self.Mesh`) (`.Mesh_2_05A2A795483B59EB3FD225AE6887AE21` (break `/Game/Data/F_Characters` _returnvalue)) false)
      (set `self.Character_Name` (`KismetStringLibrary.Conv_NameToString` _rowname)))
    (:`RowNotFound`
      (`KismetSystemLibrary.PrintString` "Personnage invalide !"))))