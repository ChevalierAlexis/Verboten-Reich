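; Dialogue manager that plays branching NPC conversations from DT_Dialogue, indexing rows through an array built on BeginPlay.
; DialogLoop checks the current line's condition via the level's single BP_Conditions and Game Instance dictionary, showing either the indexed row or a fallback.
; Lines feed the dialogue widget and add suspicion, or open a two-option choice widget that jumps to a target row.
; Player controller dispatchers drive advancing, choosing and exiting.
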(event `self.ReceiveBeginPlay`
  (bind _outrownames (`DataTableFunctionLibrary.GetDataTableRowNames` "/Game/Data/DT_Dialogue.DT_Dialogue"))
  (for _array_element _outrownames
    (`KismetArrayLibrary.Array_AddUnique` (`self.Dialog_Array`) _array_element)))

(event `Continue_Dialogue`
  (set `self.Index_Dialog` (+ (`self.Index_Dialog`) 1))
  (`self.DialogLoop`))

(event `Choice_Up`
  (bind _asbp_player_controller (`/Game/Blueprints/BPFL_MainFunctionLibrary.CastToPlayerController`))
  (for (_array_element _array_index) (`self.Dialog_Array`)
    (if (== _array_element (`.RowName` (break `DataTableRowHandle` (`.Choix_1_2_0BAF7B8947E27EB294F2748403B22644` (break `/Game/Data/F_Choix` (`.Choix_59_F0A7C4244B9AADC7965648BFA82E1636` (break `/Game/Data/F_Dialogue_Line` (`self.Current_Dialog_Line`))))))))
      (bind _output_get (set `self.Index_Dialog` _array_index))
      (`KismetSystemLibrary.PrintString` (`KismetStringLibrary.Conv_IntToString` _output_get))))
  (add `/Game/Blueprints/BP_PlayerController.OnInteraction` _asbp_player_controller (delegate `Continue_Dialogue`))
  (clear `/Game/Blueprints/BP_PlayerController.OnChoiceUp` _asbp_player_controller)
  (clear `/Game/Blueprints/BP_PlayerController.OnChoiceDown` _asbp_player_controller)
  (`/Game/Blueprints/BP_PlayerController.ChangeUI` _asbp_player_controller "NewEnumerator1")
  (`self.DialogLoop`))

(event `Choice_Down`
  (bind _asbp_player_controller (`/Game/Blueprints/BPFL_MainFunctionLibrary.CastToPlayerController`))
  (for (_array_element _array_index) (`self.Dialog_Array`)
    (if (== _array_element (`.RowName` (break `DataTableRowHandle` (`.Choix_2_4_E9045C074A895E2B67DE87934F5B3924` (break `/Game/Data/F_Choix` (`.Choix_59_F0A7C4244B9AADC7965648BFA82E1636` (break `/Game/Data/F_Dialogue_Line` (`self.Current_Dialog_Line`))))))))
      (set `self.Index_Dialog` _array_index)))
  (add `/Game/Blueprints/BP_PlayerController.OnInteraction` _asbp_player_controller (delegate `Continue_Dialogue`))
  (clear `/Game/Blueprints/BP_PlayerController.OnChoiceUp` _asbp_player_controller)
  (clear `/Game/Blueprints/BP_PlayerController.OnChoiceDown` _asbp_player_controller)
  (`/Game/Blueprints/BP_PlayerController.ChangeUI` _asbp_player_controller "NewEnumerator1")
  (`self.DialogLoop`))

(fn `Choix`
  (bind (_texte_dialogue _is_choix _is_end _suspicion_amount _anim _interlocutor _choix) (break `/Game/Data/F_Dialogue_Line` (`self.Current_Dialog_Line`)))
  (bind (_choix_1 _choix_2 _texte_1 _texte_2) (break `/Game/Data/F_Choix` _choix))
  (bind _asbp_player_controller (cast `/Game/Blueprints/BP_PlayerController` (`GameplayStatics.GetPlayerController` 0)))
  (clear `/Game/Blueprints/BP_PlayerController.OnInteraction` _asbp_player_controller)
  (`/Game/Blueprints/BP_PlayerController.ChangeUI` _asbp_player_controller "NewEnumerator2")
  (bind _asw_choix (cast `/Game/Blueprints/UI/W_Choix` (`/Game/Blueprints/BP_PlayerController.Used_Interface` _asbp_player_controller)))
  (`/Game/Blueprints/UI/W_Choix.Set_Text_Choice_Up` _asw_choix _texte_1)
  (`/Game/Blueprints/UI/W_Choix.Set_Text_Choice_Down` _asw_choix _texte_2)
  (`/Game/Blueprints/UI/W_Choix.Set_Name_Text_Choice` _asw_choix _interlocutor)
  (`/Game/Blueprints/UI/W_Choix.Set_Main_Text_Choice` _asw_choix _texte_dialogue)
  (add `/Game/Blueprints/BP_PlayerController.OnChoiceUp` _asbp_player_controller (`|CreateDelegate` :!event `Choice_Up`))
  (add `/Game/Blueprints/BP_PlayerController.OnChoiceDown` _asbp_player_controller (`|CreateDelegate` :!event `Choice_Down`)))

(fn `DialogLoop`
  (bind _asbp_player_controller (`/Game/Blueprints/BPFL_MainFunctionLibrary.CastToPlayerController`))
  (bind _asbp_game_instance (cast `/Game/Blueprints/BP_Game_Instance` (`GameplayStatics.GetGameInstance`)))
  (bind _outactors (`GameplayStatics.GetAllActorsOfClass` "/Game/Blueprints/BP_Conditions.BP_Conditions_C"))
  (if (`KismetArrayLibrary.Array_IsValidIndex` _outactors)
    (if (> (`KismetArrayLibrary.Array_Length` _outactors) 1)
      (`KismetSystemLibrary.PrintString` "Trop de BP Condition dans ce niveau !")
      (else
        (bind (_booleanvalue _suspicionvalue _iffalse _condition) (`/Game/Blueprints/BP_Conditions.Verify` (`|GetArrayItem` _outactors) (`BlueprintMapLibrary.Map_Find` (`/Game/Blueprints/BP_Game_Instance.Dict_Conditions` _asbp_game_instance) (`.Condition_63_F8AFC8AD4D5F1E088BE94681AE377B1E` (break `/Game/Data/F_Dialogue_Line` (`self.Current_Dialog_Line`))))))
        (switch `/Game/Data/E_Conditions` _condition
          (:`NewEnumerator2`
            (if (`self.End`) :!label _label
              (`/Game/Blueprints/BP_PlayerController.OnExitDialogue` _asbp_player_controller)
              (else
                (bind _returnvalue (`|GetDataTableRow` "/Game/Data/DT_Dialogue.DT_Dialogue" (`|GetArrayItem` (`self.Dialog_Array`) (`self.Index_Dialog`)))
                  (:`then`
                    (bind _output_get (set `self.Current_Dialog_Line` _returnvalue))
                    (bind _outactors_2 (`GameplayStatics.GetAllActorsOfClass` "/Game/Blueprints/BP_PNJ.BP_PNJ_C" :!label _label_2))
                    (for _array_element _outactors_2
                      (bind (_texte_dialogue _is_choix _is_end _suspicion_amount _anim _interlocutor) (break `/Game/Data/F_Dialogue_Line` _output_get))
                      (if (`KismetStringLibrary.EqualEqual_StrStr` (`/Game/Blueprints/BP_PNJ.Character_Name` _array_element) _interlocutor)
                        (bind _asw_dialogue (cast `/Game/Blueprints/UI/W_Dialogue` (`/Game/Blueprints/BP_PlayerController.Used_Interface` _asbp_player_controller) :!label _label_3))
                        (`/Game/Blueprints/UI/W_Dialogue.Set_Text_Name` _asw_dialogue _interlocutor)
                        (elif (`KismetStringLibrary.EqualEqual_StrStr` "Franz" _interlocutor)
                          (goto _label_3))))
                    (if _is_end
                      (set `self.End` true))
                    (if _is_choix
                      (`self.Choix`)
                      (else
                        (set `/Game/Blueprints/BP_PlayerController.Suspicion` (+ _suspicion_amount (`/Game/Blueprints/BP_PlayerController.Suspicion` _asbp_player_controller)) _asbp_player_controller)
                        (bind _asw_dialogue_2 (cast `/Game/Blueprints/UI/W_Dialogue` (`/Game/Blueprints/BP_PlayerController.Used_Interface` (`/Game/Blueprints/BPFL_MainFunctionLibrary.CastToPlayerController`))))
                        (`/Game/Blueprints/UI/W_Dialogue.Set_Text_Dialogue` _asw_dialogue_2 _texte_dialogue))))))))
          (:`NewEnumerator0`
            (if _booleanvalue :!label _label_4
              (goto _label)
              (else
                (bind _returnvalue_2 (`|GetDataTableRow` "/Game/Data/DT_Dialogue.DT_Dialogue" (`.RowName` (break `DataTableRowHandle` _iffalse)))
                  (:`then`
                    (set `self.Current_Dialog_Line` _returnvalue_2)
                    (goto _label_2))))))
          (:`NewEnumerator1`
            (goto _label_4)))))
    (else
      (`KismetSystemLibrary.PrintString` "Pas de BP Condition dans ce niveau"))))

(fn `PlayDialog`
  (params (DialogLine :type "DataTableRowHandle Structure"))
  (bind _asbp_player_controller (`/Game/Blueprints/BPFL_MainFunctionLibrary.CastToPlayerController`))
  (set `self.End` false)
  (`/Game/Blueprints/BP_PlayerController.EnterDialog` _asbp_player_controller)
  (add `/Game/Blueprints/BP_PlayerController.OnInteraction` _asbp_player_controller (`|CreateDelegate` :!event `Continue_Dialogue`))
  (for (_array_element _array_index) (`self.Dialog_Array`)
    (if (== _array_element (`.RowName` (break `DataTableRowHandle` DialogLine)))
      (set `self.Index_Dialog` _array_index)))
  (`self.DialogLoop`))

(fn `UserConstructionScript`)