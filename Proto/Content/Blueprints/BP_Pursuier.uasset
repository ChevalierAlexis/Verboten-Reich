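; BP_Pursuier is an armed enemy that chases the player unless Static is set, always turning its yaw toward them.
; Entering its Box volume triggers a warning shot with muzzle effect, gunfire and impact sounds, and a HUD fade-out animation.
; Entering the Close volume is fatal: it switches the UI, unbinds player input, flags DiedOnce on the game instance and reloads the level after a delay.
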(event `self.ReceiveTick`
  (params (DeltaSeconds :type "Float (single-precision)"))
  (bind _skeletalmesh (`self.SkeletalMesh`))
  (bind (_returnvalue_roll _returnvalue_pitch) (`KismetMathLibrary.BreakRotator` (`SceneComponent.K2_GetComponentRotation` _skeletalmesh)))
  (bind (_returnvalue_roll_2 _returnvalue_pitch_2 _returnvalue_yaw) (`KismetMathLibrary.BreakRotator` (`KismetMathLibrary.FindLookAtRotation` (`SceneComponent.K2_GetComponentLocation` _skeletalmesh) (`self.K2_GetActorLocation` (`Controller.K2_GetPawn` (`GameplayStatics.GetPlayerController` 0))))))
  (if (not (`self.Static`))
    (`AIBlueprintHelperLibrary.SimpleMoveToActor` (`self.GetController`) (`Controller.K2_GetPawn` (`GameplayStatics.GetPlayerController` 0))))
  (`self.K2_SetActorRotation` (`KismetMathLibrary.MakeRotator` _returnvalue_roll _returnvalue_pitch _returnvalue_yaw)))

(event `self.Box.OnComponentBeginOverlap`
  (params (OverlappedComponent :type "PrimitiveComponent Object Reference") (OtherActor :type "Actor Object Reference") (OtherComp :type "PrimitiveComponent Object Reference") (OtherBodyIndex :type Integer) (bFromSweep :type Boolean) (SweepResult :type "HitResult Structure (by ref)"))
  (cast `/Game/Blueprints/BP_Player` OtherActor)
  (`self.Warning_Shot` null)
  (`KismetSystemLibrary.Delay` 1.0))

(event `self.Close.OnComponentBeginOverlap`
  (params (OverlappedComponent :type "PrimitiveComponent Object Reference") (OtherActor :type "Actor Object Reference") (OtherComp :type "PrimitiveComponent Object Reference") (OtherBodyIndex :type Integer) (bFromSweep :type Boolean) (SweepResult :type "HitResult Structure (by ref)"))
  (cast `/Game/Blueprints/BP_Player` OtherActor)
  (`self.Shot`))

(event `Reload_Level`
  (`KismetSystemLibrary.Delay` 3.0)
  (bind _returnvalue (`GameplayStatics.GetCurrentLevelName` true))
  (`GameplayStatics.OpenLevel` (`KismetStringLibrary.Conv_StringToName` _returnvalue)))

(fn `Shot`
  (bind _asbp_player_controller (`/Game/Blueprints/BPFL_MainFunctionLibrary.CastToPlayerController`))
  (`GameplayStatics.SpawnSoundAtLocation` "/Game/Sounds/GUNAuto_Coup_de_feu_de_beretta_m12_9_mm__ID_0437__LS.GUNAuto_Coup_de_feu_de_beretta_m12_9_mm__ID_0437__LS" (`self.K2_GetActorLocation` self) (struct) 1.0 1.0 0.0 null null)
  (`/Game/Blueprints/BP_PlayerController.ChangeUI` _asbp_player_controller "NewEnumerator5")
  (clear `/Game/Blueprints/BP_PlayerController.OnMoveForward` _asbp_player_controller)
  (clear `/Game/Blueprints/BP_PlayerController.OnMoveRight` _asbp_player_controller)
  (clear `/Game/Blueprints/BP_PlayerController.OnInteraction` _asbp_player_controller)
  (clear `/Game/Blueprints/BP_PlayerController.OnMoveBackward` _asbp_player_controller)
  (clear `/Game/Blueprints/BP_PlayerController.OnPitch` _asbp_player_controller)
  (clear `/Game/Blueprints/BP_PlayerController.OnTurn` _asbp_player_controller)
  (bind _asbp_game_instance (cast `/Game/Blueprints/BP_Game_Instance` (`GameplayStatics.GetGameInstance`)))
  (set `/Game/Blueprints/BP_Game_Instance.Died_Once` true _asbp_game_instance)
  (`self.Reload_Level`))

(fn `UserConstructionScript`)

(fn `Warning_Shot`
  (params (Actor :type "Actor Object Reference"))
  (bind _skeletalmesh (`self.SkeletalMesh`))
  (`GameplayStatics.SpawnEmitterAtLocation` "/Game/Particles/P_Explosion.P_Explosion" (`SceneComponent.GetSocketLocation` _skeletalmesh "Gun") (`SceneComponent.GetSocketRotation` _skeletalmesh "Gun") (0.35 0.35 0.35))
  (bind _returnvalue (`GameplayStatics.SpawnSoundAtLocation` "/Game/Sounds/A_Bullet_Impact.A_Bullet_Impact" (`self.K2_GetActorLocation` (`GameplayStatics.GetPlayerPawn` 0)) (struct) 1.0 1.0 0.0 null null))
  (`AudioComponent.Play` _returnvalue 0.0)
  (bind _returnvalue_2 (`GameplayStatics.SpawnSoundAtLocation` "/Game/Sounds/GUNAuto_Coup_de_feu_de_beretta_m12_9_mm__ID_0437__LS.GUNAuto_Coup_de_feu_de_beretta_m12_9_mm__ID_0437__LS" (`self.K2_GetActorLocation` self) (struct) 1.0 1.0 0.0 null null))
  (`AudioComponent.Play` _returnvalue_2 0.0)
  (bind _asw_hud (cast `/Game/Blueprints/UI/W_HUD` (`/Game/Blueprints/BP_PlayerController.Used_Interface` (`/Game/Blueprints/BPFL_MainFunctionLibrary.CastToPlayerController`))))
  (`UserWidget.PlayAnimation` _asw_hud (`/Game/Blueprints/UI/W_HUD.FadeOut` _asw_hud) 0.0 1 "Forward" 1.0 false))