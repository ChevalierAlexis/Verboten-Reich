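; BP_PNJ_Egon is an NPC Blueprint that moves to a set location once the player has seen it and looked away.
; Tick runs through a Delay, throttling the check to about every 0.2 seconds unless Static is set.
; WasRecentlyRendered on the mesh latches Spotted, then triggers a move to TeleportLocation whenever the mesh is off screen.
; Spotted is never reset here, so the move repeats while unseen.
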(event `self.ReceiveTick`
  (params (DeltaSeconds :type "Float (single-precision)"))
  (`parent.ReceiveTick` DeltaSeconds)
  (`KismetSystemLibrary.Delay` 0.2)
  (if (`self.Static`)
    _
    (elif (`self.Spotted`)
      (if (not (`PrimitiveComponent.WasRecentlyRendered` (`self.Mesh`) 0.1))
        (`self.K2_SetActorLocation` (`self.Teleport_Location`)))
      (else
        (set `self.Spotted` (`PrimitiveComponent.WasRecentlyRendered` (`self.Mesh`) 0.1))))))

(fn `UserConstructionScript`
  (`parent.UserConstructionScript`))