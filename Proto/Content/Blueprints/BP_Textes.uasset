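; BP_Textes is an overlap-triggered text actor that displays string-table text to the player, either immediately or after a Read prompt and interaction.
; Its construction script fills TextArray with the table's keys.
; EnterText switches the UI, unbinds movement events and rebinds interaction before TextLoop sends the current entry to W_Textes.
; TextLoop sets End upon display, so its next call exits the dialogue.
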(event `Interact`
  (`self.EnterText`))

(event `self.ReceiveActorBeginOverlap`
  (params (OtherActor :type "Actor Object Reference"))
  (bind _asbp_player_controller (cast `/Game/Blueprints/BP_PlayerController` (`self.GetInstigatorController` OtherActor)))
  (add `/Game/Blueprints/BP_PlayerController.OnInteraction` _asbp_player_controller (delegate `Interact`))
  (if (`self.NeedInteraction`)
    (bind _asw_hud (cast `/Game/Blueprints/UI/W_HUD` (`/Game/Blueprints/BP_PlayerController.Used_Interface` _asbp_player_controller)))
    (`/Game/Blueprints/UI/W_HUD.Set_Context_Image` _asw_hud "/Game/Textures/Textures/UI/read.read")
    (else
      (`self.EnterText`))))

(event `ContinueText`
  (set `self.IndexDataBase` (+ (`self.IndexDataBase`) 1))
  (`self.TextLoop`))

(fn `EnterText`
  (bind _asbp_player_controller (`/Game/Blueprints/BPFL_MainFunctionLibrary.CastToPlayerController`))
  (set `self.End` false)
  (clear `/Game/Blueprints/BP_PlayerController.OnInteraction` _asbp_player_controller)
  (`/Game/Blueprints/BP_PlayerController.ChangeUI` _asbp_player_controller "NewEnumerator4")
  (clear `/Game/Blueprints/BP_PlayerController.OnMoveForward` _asbp_player_controller)
  (clear `/Game/Blueprints/BP_PlayerController.OnMoveRight` _asbp_player_controller)
  (add `/Game/Blueprints/BP_PlayerController.OnInteraction` _asbp_player_controller (`|CreateDelegate` :!event `ContinueText`))
  (`self.TextLoop`))

(fn `TextLoop`
  (bind _asbp_player_controller (`/Game/Blueprints/BPFL_MainFunctionLibrary.CastToPlayerController`))
  (if (`self.End`)
    (`/Game/Blueprints/BP_PlayerController.OnExitDialogue` _asbp_player_controller)
    (else
      (set `self.End` true)
      (bind _asw_textes (cast `/Game/Blueprints/UI/W_Textes` (`/Game/Blueprints/BP_PlayerController.Used_Interface` _asbp_player_controller)))
      (`/Game/Blueprints/UI/W_Textes.SetText` _asw_textes (`|GetArrayItem` (`self.Text_Array`) (`self.IndexDataBase`))))))

(fn `UserConstructionScript`
  (for _array_element (`KismetStringTableLibrary.GetKeysFromStringTable` (`self.TableID`))
    (`KismetArrayLibrary.Array_AddUnique` (`self.Text_Array`) _array_element)))