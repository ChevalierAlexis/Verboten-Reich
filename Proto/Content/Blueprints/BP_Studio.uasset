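; Item examination studio that lets the player rotate a focused item.
; Examine switches the player controller's UI and takes over its input delegates, clearing look bindings and rebinding interaction and movement axes.
; The rotate events add axis values to ItemToFocus's world yaw or pitch, and Exit_Exam calls the controller's ExitDialog to leave.
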(event `Exit_Exam`
  (`/Game/Blueprints/BP_PlayerController.Exit_Dialog` (`/Game/Blueprints/BPFL_MainFunctionLibrary.CastToPlayerController`)))

(event `Rotate`
  (params (AxisValue :type "Float (double-precision)"))
  (bind _itemtofocus (`self.ItemToFocus`))
  (bind (_returnvalue_roll _returnvalue_pitch _returnvalue_yaw) (`KismetMathLibrary.BreakRotator` (`SceneComponent.K2_GetComponentRotation` _itemtofocus)))
  (`SceneComponent.K2_SetWorldRotation` _itemtofocus (`KismetMathLibrary.MakeRotator` _returnvalue_roll _returnvalue_pitch (+ AxisValue _returnvalue_yaw)) false false))

(event `RotateUpDown`
  (params (AxisValue :type "Float (double-precision)"))
  (bind _itemtofocus (`self.ItemToFocus`))
  (bind (_returnvalue_roll _returnvalue_pitch _returnvalue_yaw) (`KismetMathLibrary.BreakRotator` (`SceneComponent.K2_GetComponentRotation` _itemtofocus)))
  (`SceneComponent.K2_SetWorldRotation` _itemtofocus (`KismetMathLibrary.MakeRotator` _returnvalue_roll (+ AxisValue _returnvalue_pitch) _returnvalue_yaw) false false))

(fn `Examine`
  (bind _asbp_player_controller (cast `/Game/Blueprints/BP_PlayerController` (`GameplayStatics.GetPlayerController` 0)))
  (clear `/Game/Blueprints/BP_PlayerController.OnInteraction` _asbp_player_controller)
  (add `/Game/Blueprints/BP_PlayerController.OnInteraction` _asbp_player_controller (`|CreateDelegate` :!event `Exit_Exam`))
  (`/Game/Blueprints/BP_PlayerController.ChangeUI` _asbp_player_controller "NewEnumerator3")
  (clear `/Game/Blueprints/BP_PlayerController.OnMoveForward` _asbp_player_controller)
  (clear `/Game/Blueprints/BP_PlayerController.OnMoveRight` _asbp_player_controller)
  (clear `/Game/Blueprints/BP_PlayerController.OnTurn` _asbp_player_controller)
  (clear `/Game/Blueprints/BP_PlayerController.OnPitch` _asbp_player_controller)
  (clear `/Game/Blueprints/BP_PlayerController.GamepadOnPitch` _asbp_player_controller)
  (clear `/Game/Blueprints/BP_PlayerController.GamepadOnTurn` _asbp_player_controller)
  (add `/Game/Blueprints/BP_PlayerController.OnMoveRight` _asbp_player_controller (`|CreateDelegate` :!event `Rotate`))
  (add `/Game/Blueprints/BP_PlayerController.OnMoveForward` _asbp_player_controller (`|CreateDelegate` :!event `RotateUpDown`)))

(fn `UserConstructionScript`)